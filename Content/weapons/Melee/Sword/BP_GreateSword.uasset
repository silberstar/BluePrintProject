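; Greatsword melee weapon Blueprint that deals combo-based damage through a capsule hitbox, extending inherited combo, attack and collision events.
; Mesh and capsule collision start disabled; OnCollision and OffCollision toggle only the capsule during play.
; Capsule overlaps send damage from WeaponDamageComponent for the current ComboCount, skipping actors of the owner's class.
; StartCombo and EndAttack call the parent, then start or end the attack on that component.
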(event OnComponentBeginOverlap(Capsule)
  (params (OverlappedComponent :type Primitive%20Component%20Object%20Reference) (OtherActor :type Actor%20Object%20Reference) (OtherComp :type Primitive%20Component%20Object%20Reference) (OtherBodyIndex :type Integer) (bFromSweep :type Boolean) (SweepResult :type Hit%20Result%20Structure%20%28by%20ref%29))
  (bind _returnvalue (Default|GetComboDamage (Variables|Default|GetWeaponDamageComponent) (Variables|Default|GetComboCount)))
  (if (!= (Utilities|GetClass OtherActor) (Utilities|GetClass (Components|GetOwner)))
    (CallFunction|SendDamage OtherActor _returnvalue)))

(event Collision|EventActorBeginOverlap
  (params (OtherActor :type Actor%20Object%20Reference)))

(event EventStartCombo
  (|CallParentFunction)
  (Default|StartAttack (Variables|Default|GetWeaponDamageComponent)))

(event EventTick
  (params (DeltaSeconds :type Float%20%28single-precision%29)))

(event EventEndAttack
  (|CallParentFunction)
  (Default|EndAttack (Variables|Default|GetWeaponDamageComponent)))

(event EventOnCollision
  (params (FistCollision :type E_FistCollisionType%20Enum :default "NewEnumerator0"))
  (|CallParentFunction FistCollision)
  (Collision|SetCollisionEnabled (Variables|Default|GetCapsule) "QueryAndPhysics"))

(event EventOffCollision
  (|CallParentFunction)
  (Collision|SetCollisionEnabled (Variables|Default|GetCapsule) "NoCollision"))

(event EventBeginPlay
  (|CallParentFunction)
  (Collision|SetCollisionEnabled (Variables|Default|GetSkeletalMesh) "NoCollision"))

(fn ConstructionScript)