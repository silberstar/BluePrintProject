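; Melee dagger weapon Blueprint that deals combo-scaled damage on capsule overlap and destroys itself when it has no valid owner.
; Collision events toggle the hit capsule; overlaps with actors of a different class than the owner send damage from WeaponDamageComponent's combo value times Power.
; Attack start/end events extend parent logic and notify the damage component.
; Transformation events play forward or reverse bayonet-change montages on the weapon mesh.
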(event OnComponentBeginOverlap(Capsule)
  (params (OverlappedComponent :type Primitive%20Component%20Object%20Reference) (OtherActor :type Actor%20Object%20Reference) (OtherComp :type Primitive%20Component%20Object%20Reference) (OtherBodyIndex :type Integer) (bFromSweep :type Boolean) (SweepResult :type Hit%20Result%20Structure%20%28by%20ref%29))
  (bind _returnvalue (Default|GetComboDamage (Variables|Default|GetWeaponDamageComponent) (Variables|Default|GetComboCount)))
  (if (!= (Utilities|GetClass OtherActor) (Utilities|GetClass (Components|GetOwner)))
    (CallFunction|SendDamage OtherActor (* _returnvalue (Variables|Default|GetPower)))
    (bind _asbp_player_armored (Utilities|Casting|CastToBP_Player_Armored OtherActor))
    (Development|PrintString (Utilities|GetDisplayName _asbp_player_armored))))

(event Custom|CustomEvent
  (|CallParentFunction)
  (Default|StartAttack (Variables|Default|GetWeaponDamageComponent)))

(event Custom|CustomEvent_1
  (|CallParentFunction)
  (Default|EndAttack (Variables|Default|GetWeaponDamageComponent)))

(event EventBeginPlay
  (Collision|SetCollisionEnabled (Variables|Default|GetSkeletalMesh) "NoCollision"))

(event Collision|EventActorBeginOverlap
  (params (OtherActor :type Actor%20Object%20Reference)))

(event EventTick
  (params (DeltaSeconds :type Float%20%28single-precision%29))
  (Utilities|IsValid (Components|GetOwner)
    (:Is%20Not%20Valid
      (Actor|DestroyActor))))

(event EventOnCollision
  (params (FistCollision :type E_FistCollisionType%20Enum :default "NewEnumerator0"))
  (Collision|SetCollisionEnabled (Variables|Default|GetCapsule) "QueryAndPhysics"))

(event EventOffCollision
  (Collision|SetCollisionEnabled (Variables|Default|GetCapsule) "NoCollision"))

(event EventWeaponTransformation
  (|CallParentFunction)
  (Animation|Montage|PlayMontage (Variables|Default|GetSkeletalMesh) "/Game/Character/Animations/CeangeWeapon/Dager/RifleLongSword__BayonetChange__Montage.RifleLongSword__BayonetChange__Montage"))

(event EventWeaponTransformationRevers
  (|CallParentFunction)
  (Animation|Montage|PlayMontage (Variables|Default|GetSkeletalMesh) "/Game/Character/Animations/CeangeWeapon/Dager/RifleLongSword__BayonetChange__Montage_Reverse.RifleLongSword__BayonetChange__Montage_Reverse"))

(fn ConstructionScript)

(fn SetCurrentWeapon
  (params (NewWeapon :type BP%20Weapon%20Object%20Reference))
  (return false))

(fn GetCurrentWeapon
  (return 0))