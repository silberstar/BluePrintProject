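; Long sword weapon that pairs with a spawned, attached BP_Dager1 and transforms between sword and gun modes via montages.
; Melee overlaps deal combo damage: normal grip enables the capsule and dagger collision, while Mordhau grip enables a box that adds Power.
; Tick drives gunfire with a burst-then-faster cadence, camera shake and dagger-mesh rotation.
; Each shot spends ammo, spawns a bullet and applies damage through a line trace.
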(event OnComponentBeginOverlap(Capsule)
  (params (OverlappedComponent :type Primitive%20Component%20Object%20Reference) (OtherActor :type Actor%20Object%20Reference) (OtherComp :type Primitive%20Component%20Object%20Reference) (OtherBodyIndex :type Integer) (bFromSweep :type Boolean) (SweepResult :type Hit%20Result%20Structure%20%28by%20ref%29))
  (bind _returnvalue (Default|GetComboDamage (Variables|Default|GetWeaponDamageComponent) (Variables|Default|GetComboCount)))
  (if (!= (Utilities|GetClass OtherActor) (Utilities|GetClass (Components|GetOwner)))
    (CallFunction|SendDamage OtherActor _returnvalue)))

(event OnComponentBeginOverlap(Box)
  (params (OverlappedComponent :type Primitive%20Component%20Object%20Reference) (OtherActor :type Actor%20Object%20Reference) (OtherComp :type Primitive%20Component%20Object%20Reference) (OtherBodyIndex :type Integer) (bFromSweep :type Boolean) (SweepResult :type Hit%20Result%20Structure%20%28by%20ref%29))
  (bind _returnvalue (Default|GetComboDamage (Variables|Default|GetWeaponDamageComponent) (Variables|Default|GetComboCount)))
  (if (!= (Utilities|GetClass OtherActor) (Utilities|GetClass (Components|GetOwner)))
    (CallFunction|SendDamage OtherActor (+ _returnvalue (Variables|Default|GetPower)))))

(event Custom|BaisicGrip
  (Variables|Default|SetTurnOn false))

(event Custom|MordHau
  (Variables|Default|SetTurnOn true))

(event EventBeginPlay
  (|CallParentFunction)
  (bind _returnvalue (Game|SpawnActorfromClass "/Game/weapons/Melee/Sword/BP_Dager1.BP_Dager1_C" (Math|Transform|MakeTransform "0, 0, 0") "Undefined" self 0))
  (Collision|SetCollisionEnabled (Variables|Default|GetSkeletalMesh) "NoCollision")
  (bind _output_get (Variables|Default|SetSword _returnvalue))
  (Transformation|AttachComponentToComponent _output_get (Variables|Default|GetSkeletalMesh) "DaggerAttach" "KeepRelative" "KeepRelative" "KeepRelative" true))

(event Collision|EventActorBeginOverlap
  (params (OtherActor :type Actor%20Object%20Reference)))

(event EventTick
  (params (DeltaSeconds :type Float%20%28single-precision%29))
  (|IsShooting))

(event EventOnCollision
  (params (FistCollision :type E_FistCollisionType%20Enum :default "NewEnumerator0"))
  (|CallParentFunction FistCollision)
  (if (not (Variables|Default|GetTurnOn))
    (Collision|SetCollisionEnabled (Variables|Default|GetCapsule) "QueryAndPhysics")
    (Default|OnCollision (Variables|Default|GetSword) "NewEnumerator0")
    (else
      (Collision|SetCollisionEnabled (Variables|Default|GetBox) "QueryAndPhysics"))))

(event EventOffCollision
  (|CallParentFunction)
  (Collision|SetCollisionEnabled (Variables|Default|GetCapsule) "NoCollision")
  (Default|OffCollision (Variables|Default|GetSword)))

(event EventReload
  (|CallParentFunction))

(event EventEndAttack
  (|CallParentFunction)
  (Default|EndAttack (Variables|Default|GetWeaponDamageComponent)))

(event EventWeaponTransformation
  (|CallParentFunction)
  (bind _gun (Timeline|TransformTimeLine PlayFromStart)
    (:Update
      (bind _asbp_player (Utilities|Casting|CastToBP_Player (Components|GetOwner)))
      (Variables|/Game/Player/BP_Player.BP_Player_C|SetGunMode _asbp_player _gun)
      (Variables|Default|SetMode _gun)
      (Animation|Montage|PlayMontage (Variables|Default|GetSkeletalMesh) "/Game/Character/Animations/CeangeWeapon/Anim_CangeGun_Montage.Anim_CangeGun_Montage"
        (:then
          (Default|WeaponTransformation (Variables|Default|GetSword)))))))

(event EventWeaponTransformationRevers
  (|CallParentFunction)
  (Animation|Montage|PlayMontage (Variables|Default|GetSkeletalMesh) "/Game/Character/Animations/CeangeWeapon/Anim_CangeSword_Montage.Anim_CangeSword_Montage"
    (:then
      (Default|WeaponTransformationRevers (Variables|Default|GetSword)))))

(event EventStartCombo
  (|CallParentFunction)
  (Default|StartAttack (Variables|Default|GetWeaponDamageComponent)))

(fn ConstructionScript)