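; BP_Melee is a melee weapon Blueprint that runs montage-based combo attacks for its owning character.
; On BeginPlay it loads rows matching its MeleeType from the owner's MeleeData table, supplying each step's montage, play rate and movement permission.
; Attack starts or queues combos, which PlayNextCombo advances, and enables shooting on transformed player weapons.
; SendDamage tracks hit actors and triggers camera shake, brief time-dilation hit-stop and a last-combo particle.
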(event Custom|DamageEffect
  (if (Variables|Default|GetLastCombo)
    (Effects|SpawnEmitteratLocation "/Game/Particles/P_LastCombo.P_LastCombo" (Transformation|GetActorLocation)))
  (|HitCameraShake)
  (Utilities|Time|SetGlobalTimeDilation 0.15)
  (Utilities|FlowControl|Delay 0.015)
  (Utilities|Time|SetGlobalTimeDilation 1.0))

(event Custom|PlayNextCombo
  ;[1 1 1] 콤보연결 성공
  (if (Variables|Default|GetSucceedCombo)
    (Variables|Default|SetSucceedCombo false)
    (Math|Integer|IncrementInt (Variables|Default|GetComboCount)
      (:%20%20
        (CallFunction|PlayComboMontage)
        (Variables|Default|SetLastCombo (== (Variables|Default|GetComboCount) (- (Utilities|Array|Length (Variables|Default|GetMeleeDatas)) 1)))))))

(event EventBeginPlay
  ;[1 1 1] 데이터테이블 읽어오기
  (|CallParentFunction)
  (bind _asbp_character (Utilities|Casting|CastToBP_Character (Components|GetOwner)))
  (Variables|Default|SetDataTable (Variables|/Game/Character/BP_Character.BP_Character_C|GetMeleeData _asbp_character))
  (Utilities|FlowControl|Sequence
    (:then_0
      (|ReadDataTable))))

(event Collision|EventActorBeginOverlap
  (params (OtherActor :type Actor%20Object%20Reference))
  (|CallParentFunction OtherActor) ; 지금 이 노드는 비활성 상태입니다. \n핀을 끌어서 다른 노드를 연결하면 활성화됩니다.
)

(event EventTick
  (params (DeltaSeconds :type Float%20%28single-precision%29))
  (|CallParentFunction DeltaSeconds) ; 지금 이 노드는 비활성 상태입니다. \n핀을 끌어서 다른 노드를 연결하면 활성화됩니다.
)

(event EventAttack
  ;[1 1 1] 공격 이벤트
  (|CallParentFunction)
  (Utilities|FlowControl|Sequence
    (:then_0
      (|ComboEvent))
    (:then_1
      (|ShootingEvent))))

(event EventEndAttack
  ;[1 1 1] 공격 종료
  (|CallParentFunction)
  (CallFunction|SetStateIdling)
  (Variables|Default|SetComboCount 0)
  (CallFunction|SetCanMove true)
  (Variables|Default|SetSucceedCombo false)
  (Variables|Default|SetLastCombo false)
  (CallFunction|EndCombo))

(fn ConstructionScript
  (|CallParentFunction))

(fn PlayComboMontage
  (bind _returnvalue (Components|GetOwner))
  (bind _meleedatas (Variables|Default|GetMeleeDatas))
  (bind _combocount (Variables|Default|GetComboCount))
  (bind _output (Utilities|Array|Get(acopy) _meleedatas _combocount))
  (bind _ascharacter (Utilities|Casting|CastToCharacter _returnvalue))
  (Animation|PlayAnimMontage _ascharacter (.montage _output) (.playlate _output) (.startsection _output))
  (CallFunction|SetCanMove (.canmove _output))
  (bind _asbp_player (Utilities|Casting|CastToBP_Player _returnvalue))
  (Utilities|IsValid _asbp_player
    (:Is%20Valid
      (Default|Action _asbp_player))
    (:Is%20Not%20Valid
      (Development|PrintString "Hello"))))

(fn OnCollision
  (params (FistCollision :type E_FistCollisionType%20Enum :default "NewEnumerator0")))

(fn OffCollision
  (Utilities|Array|Clear (Variables|Default|GetHitedActors)))

(fn SendDamage
  (params (OtherActor :type Actor%20Object%20Reference) (Damage :type Float%20%28single-precision%29))
  (bind _array_element (Utilities|Array|ForEachLoopwithBreak (Variables|Default|GetHitedActors) :!label _label)
    (:LoopBody
      (if (== _array_element OtherActor)
        (LocalVariables|SetEverHitedActor false)
        (goto _label Break)))
    (:Completed
      (if (not (LocalVariables|GetEverHitedActor))
        (Utilities|Array|Add (Variables|Default|GetHitedActors) OtherActor)
        (bind _result (|CallParentFunction OtherActor Damage))
        (Utilities|Casting|CastToCharacter OtherActor)
        (if _result
          (CallFunction|DamageEffect)
          (return _result))))))

(fn StartCombo)

(fn EndCombo)