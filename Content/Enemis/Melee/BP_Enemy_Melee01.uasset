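; BP_Enemy_Melee01 is a melee enemy child Blueprint that carries a greatsword and two longswords.
; It overrides equip and unequip events to set or clear the current weapon and switch combat type.
; Attach and Detach move all three weapon meshes between hand and holster sockets.
; CurrentWeaponType always selects the greatsword, as its WeaponStyle branches are disconnected from the function entry.
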(event EventBeginPlay
  (|CallParentFunction) ; 지금 이 노드는 비활성 상태입니다. \n핀을 끌어서 다른 노드를 연결하면 활성화됩니다.
)

(event Collision|EventActorBeginOverlap
  (params (OtherActor :type Actor%20Object%20Reference))
  (|CallParentFunction OtherActor) ; 지금 이 노드는 비활성 상태입니다. \n핀을 끌어서 다른 노드를 연결하면 활성화됩니다.
)

(event EventDetach
  (bind _mesh (Variables|Character|GetMesh))
  (|CallParentFunction)
  (Transformation|AttachComponentToComponent (Variables|Default|GetLongSword1) _mesh "Holster_TwoHended" "KeepRelative" "KeepRelative" "KeepRelative" true)
  (Transformation|AttachComponentToComponent (Variables|Default|GetGrateSword) _mesh "Holster_GreateSword" "KeepRelative" "KeepRelative" "KeepRelative" true)
  (Transformation|AttachComponentToComponent (Variables|Default|GetLongSword2) _mesh "Holster_Sword" "KeepRelative" "KeepRelative" "KeepRelative" true)
  (Variables|Default|SetAttached false))

(event EventTick
  (params (DeltaSeconds :type Float%20%28single-precision%29))
  (|CallParentFunction DeltaSeconds) ; 지금 이 노드는 비활성 상태입니다. \n핀을 끌어서 다른 노드를 연결하면 활성화됩니다.
)

(event EventEquipped
  (|CallParentFunction)
  (|CurrentWeaponType)
  (Variables|Default|SetCombatType "NewEnumerator1"))

(event EventUnEquipped
  (|CallParentFunction)
  (CallFunction|SetCurrentWeapon)
  (Variables|Default|SetCombatType "NewEnumerator0"))

(event EventAttach
  (bind _mesh (Variables|Character|GetMesh))
  (|CallParentFunction)
  (Transformation|AttachComponentToComponent (Variables|Default|GetLongSword1) _mesh "hand_r_Weapon" "KeepRelative" "KeepRelative" "KeepRelative" true)
  (Transformation|AttachComponentToComponent (Variables|Default|GetGrateSword) _mesh "hand_GrateSword" "KeepRelative" "KeepRelative" "KeepRelative" true)
  (Variables|Default|SetAttached true))

(fn ConstructionScript
  (|CallParentFunction))