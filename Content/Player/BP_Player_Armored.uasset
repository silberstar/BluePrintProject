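; Armored player character that transforms between a bot and a gravity-free jet vehicle on K.
; A timeline plays forward or in reverse through staged collapsed graphs that move armor and wings, swap anim classes and reconfigure weapon, movement and camera lag.
; Parent action overrides mirror montages onto armor meshes, mostly only in bot form.
; With a sword, F toggles a timeline-animated shield built from wing parts on a spring arm.
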(event Custom|BotMode
  (Variables|Default|SetChanged false)
  (bind (_direction _mode _wingtarget _rotate _wingtransform _wingrotetor _armortransform _새_트랙_0 _새_트랙_1) (Timeline|TransformTimeline Reverse)
    (:Update
      (|Transform_01 _mode _wingtarget _rotate _wingtransform _wingrotetor _armortransform _새_트랙_0 _새_트랙_1)
      (if (Variables|Default|GetChanged)
        (|Transform_02 :!label _label)
        (if (Variables|Default|GetChanged)
          (|Transtorm_03 :!label _label_2)
          (if (== (Variables|Default|GetMode) 0.0)
            (Class|SkeletalMeshComponent|SetAnimClass (Variables|Character|GetMesh) "/Game/Player/ABP_Player_Armored.ABP_Player_Armored_C")
            (Variables|Default|SetShildEquipped false))
          (else
            (goto _label_2 execute2)))
        (else
          (goto _label execute2))))))

(event Custom|VhicleMode
  (Variables|Default|SetChanged true)
  (bind (_direction _mode _wingtarget _rotate _wingtransform _wingrotetor _armortransform _새_트랙_0 _새_트랙_1) (Timeline|TransformTimeline PlayFromStart)
    (:Update
      (|Transform_01 _mode _wingtarget _rotate _wingtransform _wingrotetor _armortransform _새_트랙_0 _새_트랙_1)
      (if (Variables|Default|GetChanged)
        (|Transform_02 :!label _label)
        (if (Variables|Default|GetChanged)
          (|Transtorm_03 :!label _label_2)
          (if (== (Variables|Default|GetMode) 0.0)
            (Class|SkeletalMeshComponent|SetAnimClass (Variables|Character|GetMesh) "/Game/Player/ABP_Player_Armored.ABP_Player_Armored_C")
            (Variables|Default|SetShildEquipped false))
          (else
            (goto _label_2 execute2)))
        (else
          (goto _label execute2))))))

(event EventBeginPlay
  (|CallParentFunction)
  (Utilities|FlowControl|Sequence
    (:then_0
      (|BoneHiden))))

(event Collision|EventActorBeginOverlap
  (params (OtherActor :type Actor%20Object%20Reference))
  (|CallParentFunction OtherActor) ; 지금 이 노드는 비활성 상태입니다. \n핀을 끌어서 다른 노드를 연결하면 활성화됩니다.
)

(event EventTick
  (params (DeltaSeconds :type Float%20%28single-precision%29))
  (|CallParentFunction DeltaSeconds) ; 지금 이 노드는 비활성 상태입니다. \n핀을 끌어서 다른 노드를 연결하면 활성화됩니다.
)

(event EventDead
  (|CallParentFunction))

(event Input|KeyboardEvents|K
  (params (Key :type Key%20Structure :default "None"))
  (bind _mode (Variables|Default|GetMode))
  (:Pressed
    (if (and (Variables|Default|GetChange) (Variables|Default|GetCanMove))
      (CallFunction|UnEquippedSword)
      (Transformation|AttachComponentToComponent (Variables|Default|GetSpringArmWing) (Variables|Character|GetMesh) "Root" "KeepRelative" "KeepRelative" "KeepRelative" true)
      (Utilities|FlowControl|Sequence
        (:then_0
          (if (not (<= _mode 0.0))
            (CallFunction|BotMode)))
        (:then_1
          (if (not (>= _mode 1e+02))
            (CallFunction|VhicleMode)))))))

(fn ConstructionScript
  (|CallParentFunction))

(event Custom|Montage%20Play
  (params (Montage :type Anim%20Montage%20Object%20Reference) (PlayRate :type Float%20%28single-precision%29) (StartingSection :type Name))
  (Animation|Montage|PlayMontage (Variables|Default|Getvambrace) Montage PlayRate 0.0 StartingSection
    (:then
      (Animation|Montage|PlayMontage (Variables|Default|Getpoleyn) Montage PlayRate 0.0 StartingSection))))

(event Custom|ShildEquip
  (Variables|Default|SetShildEquipped true)
  (Variables|/Script/Engine.SpringArmComponent|SetCameraLagSpeed (Variables|Default|GetSpringArmWing) 2e+01)
  (Transformation|AttachComponentToComponent (Variables|Default|GetSpringArmWing) (Variables|Character|GetMesh) "lowerarm_l_Shild" "KeepRelative" "KeepRelative" "KeepRelative" true)
  (Rendering|Material|SetMaterial (Variables|Default|GetWing1) 2 "/Game/Character/Weapons/SwordPistol/Material/Jem/MAT_Crystal_Inst.MAT_Crystal_Inst")
  (CallFunction|ShildAttach)
  (bind (_direction _shild _visor _shildlocation _shiuldrotation _shildbottomlocation _새_트랙_0 _새_트랙_1) (Timeline|타임라인_0_0 PlayFromStart)
    (:Update
      (Variables|Default|SetWingMode _shild)
      (Transformation|SetRelativeTransform (Variables|Default|GetWing) (Math|Transform|MakeTransform _shildlocation "0,90.000000,90.000000" "0.770000,0.770000,0.770000") true false)
      (Transformation|SetRelativeTransform (Variables|Default|GetWing1) (Math|Transform|MakeTransform (Math|Vector|MakeVector (.X (Math|Vector|BreakVector _shildlocation)) (* (.Y (Math|Vector|BreakVector _shildlocation)) -1.0) (.Z (Math|Vector|BreakVector _shildlocation))) "0,90.000000,90.000000" "-0.770000,0.770000,0.770000") true false)
      (Transformation|SetRelativeTransform (Variables|Default|GetTail%20Wing) (Math|Transform|MakeTransform _shildbottomlocation (Math|Rotator|MakeRotator (.x _shiuldrotation) (.y _shiuldrotation) (.z _shiuldrotation)) "-0.770000,0.770000,0.770000") true false)
      (Transformation|SetRelativeTransform (Variables|Default|GetStaticMesh1) (Math|Transform|MakeTransform _새_트랙_0 (Math|Rotator|MakeRotator (.X (Math|Vector|BreakVector _새_트랙_1)) (.Y (Math|Vector|BreakVector _새_트랙_1)) (.Z (Math|Vector|BreakVector _새_트랙_1))) "0.770000,0.770000,0.770000") false false))))

(event Custom|Shild%20UnEquip
  (Variables|Default|SetShildEquipped false)
  (Variables|/Script/Engine.SpringArmComponent|SetCameraLagSpeed (Variables|Default|GetSpringArmWing) 8.0)
  (Transformation|AttachComponentToComponent (Variables|Default|GetSpringArmWing) (Variables|Character|GetMesh) "" "KeepRelative" "KeepRelative" "KeepRelative" true)
  (Rendering|Material|SetMaterial (Variables|Default|GetWing1) 2 "/Game/Materials/MAT_Invisible.MAT_Invisible")
  (CallFunction|ShildDettach)
  (bind (_direction _shild _visor _shildlocation _shiuldrotation _shildbottomlocation _새_트랙_0 _새_트랙_1) (Timeline|타임라인_0_0 Reverse)
    (:Update
      (Variables|Default|SetWingMode _shild)
      (Transformation|SetRelativeTransform (Variables|Default|GetWing) (Math|Transform|MakeTransform _shildlocation "0,90.000000,90.000000" "0.770000,0.770000,0.770000") true false)
      (Transformation|SetRelativeTransform (Variables|Default|GetWing1) (Math|Transform|MakeTransform (Math|Vector|MakeVector (.X (Math|Vector|BreakVector _shildlocation)) (* (.Y (Math|Vector|BreakVector _shildlocation)) -1.0) (.Z (Math|Vector|BreakVector _shildlocation))) "0,90.000000,90.000000" "-0.770000,0.770000,0.770000") true false)
      (Transformation|SetRelativeTransform (Variables|Default|GetTail%20Wing) (Math|Transform|MakeTransform _shildbottomlocation (Math|Rotator|MakeRotator (.x _shiuldrotation) (.y _shiuldrotation) (.z _shiuldrotation)) "-0.770000,0.770000,0.770000") true false)
      (Transformation|SetRelativeTransform (Variables|Default|GetStaticMesh1) (Math|Transform|MakeTransform _새_트랙_0 (Math|Rotator|MakeRotator (.X (Math|Vector|BreakVector _새_트랙_1)) (.Y (Math|Vector|BreakVector _새_트랙_1)) (.Z (Math|Vector|BreakVector _새_트랙_1))) "0.770000,0.770000,0.770000") false false))))

(event EventAttach
  (if (not (Variables|Default|GetChanged))
    (|CallParentFunction)
    (CallFunction|ShildUnEquip)))

(event EventShooter
  (if (not (Variables|Default|GetChanged))
    (|CallParentFunction)
    (CallFunction|ShildUnEquip)))

(event EventCrouching
  (if (not (Variables|Default|GetChanged))
    (|CallParentFunction)
    (Utilities|FlowControl|FlipFlop
      (:A
        (CallFunction|MontagePlay (Variables|Default|GetCrouchingAnimMontage) 1.0 "None"))
      (:B
        (if (not (not (Variables|Default|GetIsProning)))
          (CallFunction|MontagePlay (Variables|Default|GetStandMontage) 1.0 "None"))))))

(event EventBackStep
  (if (not (Variables|Default|GetChanged))
    (|CallParentFunction)
    (CallFunction|MontagePlay (Variables|Default|GetBackstepMontage) 1.0 "None")))

(event EventEquippSword
  (if (not (Variables|Default|GetChanged))
    (|CallParentFunction)
    (CallFunction|MontagePlay (Variables|Default|GetDrawMontage) 0.8 "None")
    (Variables|Default|SetVisorOpen 0.0)
    (Rendering|Material|SetMaterial (Variables|Default|GetVisor) 3 "/Game/Character/Weapons/SwordPistol/Material/Jem/MAT_Crystal_Inst.MAT_Crystal_Inst")))

(event EventUnEquippSword
  (if (not (Variables|Default|GetChanged))
    (|CallParentFunction)
    (CallFunction|MontagePlay (Variables|Default|GetSheathMontage) 1.0 "None")
    (Variables|Default|SetVisorOpen 1e+02)
    (Rendering|Material|SetMaterial (Variables|Default|GetVisor) 3 "/Game/Materials/MAT_Invisible.MAT_Invisible")
    (CallFunction|ShildUnEquip)))

(event EventReLoad
  (|CallParentFunction)
  (if (not (Variables|Default|GetChanged))
    (CallFunction|MontagePlay (Variables|Default|GetReLoadMontage) 1.0 "None")))

(event EventAction
  (|CallParentFunction)
  (bind _currentweapon (CallFunction|GetCurrentWeapon))
  (bind _asbp_melee (Utilities|Casting|CastToBP_Melee _currentweapon)
    (:then
      (CallFunction|MontagePlay (.montage (Utilities|Array|Get(acopy) (Variables|/Game/weapons/Melee/BP_Melee.BP_Melee_C|GetMeleeDatas _asbp_melee) (Variables|/Game/weapons/Melee/BP_Melee.BP_Melee_C|GetComboCount _asbp_melee))) (.playlate (Utilities|Array|Get(acopy) (Variables|/Game/weapons/Melee/BP_Melee.BP_Melee_C|GetMeleeDatas _asbp_melee) (Variables|/Game/weapons/Melee/BP_Melee.BP_Melee_C|GetComboCount _asbp_melee))) (.startsection (Utilities|Array|Get(acopy) (Variables|/Game/weapons/Melee/BP_Melee.BP_Melee_C|GetMeleeDatas _asbp_melee) (Variables|/Game/weapons/Melee/BP_Melee.BP_Melee_C|GetComboCount _asbp_melee)))))
    (:CastFailed
      (Utilities|Casting|CastToBP_Magic _currentweapon))))

(event EventSetRollingDirection
  (if (not (Variables|Default|GetChanged))
    (|CallParentFunction)
    (CallFunction|MontagePlay (Variables|Default|GetRollMontage) 1.5 "None")))

(event EventProning
  (if (not (Variables|Default|GetChanged))
    (|CallParentFunction)
    (CallFunction|MontagePlay (Variables|Default|GetProningMontage) 1.0 "None")))

(event Input|KeyboardEvents|F
  (params (Key :type Key%20Structure :default "None"))
  (:Pressed
    (if (and (not (Variables|Default|GetChanged)) (Variables|Default|GetCanMove))
      (switch Utilities|FlowControl|Switch|SwitchonE_CombatStyle (Variables|Default|GetCombatType)
        (:NewEnumerator0
          (CallFunction|ShildUnEquip :!label _label))
        (:NewEnumerator1
          (bind _asbp_melee (Utilities|Casting|CastToBP_Melee (Variables|Default|GetCurrentWeapon)))
          (switch Utilities|FlowControl|Switch|SwitchonE_MeleeType (Variables|/Game/weapons/Melee/BP_Melee.BP_Melee_C|GetMeleeType _asbp_melee)
            (:NewEnumerator0
              (goto _label))
            (:NewEnumerator1
              (goto _label))
            (:NewEnumerator2
              (if (not (Variables|Default|GetShildEquipped))
                (CallFunction|ShildEquip)
                (else
                  (CallFunction|ShildUnEquip))))
            (:NewEnumerator3
              (goto _label))
            (:NewEnumerator4
              (goto _label))))
        (:NewEnumerator2
          (goto _label))))))

(event Custom|ShildDettach
  (Transformation|AttachComponentToComponent (Variables|Default|GetStaticMesh1) (Variables|Default|GetWast) "ButtPlate소켓" "KeepRelative" "KeepRelative" "KeepRelative" true))

(event Custom|ShildAttach
  (Transformation|AttachComponentToComponent (Variables|Default|GetStaticMesh1) (Variables|Default|GetSpringArmWing) "SpringEndpoint" "SnapToTarget" "SnapToTarget" "KeepRelative" true))

(event Custom|SetBone
  (params (타깃 :type Scene%20Component%20Object%20Reference) (SocketName :type Name))
  (Transformation|AttachComponentToComponent 타깃 (Variables|Character|GetMesh) SocketName "KeepRelative" "KeepRelative" "KeepRelative" true))